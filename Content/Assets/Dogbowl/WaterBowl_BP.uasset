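; Dog water bowl actor that tracks a water level, drained as a Mufn actor drinks from it.
; The level starts full at BeginPlay.
; When DrinkRange begins an overlap and contains a MufnActor, a delay loop lowers the level every two seconds while the VRPawn's IsMovingToWater flag is set.
; The loop has no end-overlap exit or lower limit on the level.
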(event OnComponentBeginOverlap(DrinkRange)
  (params (OverlappedComponent :type Primitive%20Component%20Object%20Reference) (OtherActor :type Actor%20Object%20Reference) (OtherComp :type Primitive%20Component%20Object%20Reference) (OtherBodyIndex :type Integer) (bFromSweep :type Boolean) (SweepResult :type Hit%20Result%20Structure%20%28by%20ref%29))
  ;[1 1 1] Drinks every 2 seconds when in range and trying to drink
  (if (> (Math|Conversions|ToByte(Integer) (Utilities|Array|Length (Collision|GetOverlappingActors OverlappedComponent (Utilities|GetClass (Variables|Default|GetMufnActor)) :!class /Script/Engine.PrimitiveComponent))) 0)
    (bind _asvrpawn (Utilities|Casting|CastToVRPawn (Game|Player|GetPlayerPawn 0)))
    (while (Variables|/Game/VRTemplate/Blueprints/VRPawn.VRPawn_C|GetisMovingToWater _asvrpawn)
      (Utilities|FlowControl|Delay 2.0)
      (Variables|Default|SetWaterLevel (- (Variables|Default|GetWaterLevel) 10)))))

(event EventBeginPlay
  (Variables|Default|SetWaterLevel 100))

(event Collision|EventActorBeginOverlap
  (params (OtherActor :type Actor%20Object%20Reference)))

(event EventTick
  (params (DeltaSeconds :type Float%20%28single-precision%29)))

(fn ConstructionScript)